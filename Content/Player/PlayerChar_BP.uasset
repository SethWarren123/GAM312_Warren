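; Player character Blueprint that holds Health, Hunger and Stamina stats plus a resource inventory array.
; Every Tick it appends these values into one debug string and shows it with Print String, reading the first three array slots as Wood, Stone and Berry.
; The graphs contain no logic that changes the stats or resources, and the construction script is empty.
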(event `self.ReceiveTick`
  (params (DeltaSeconds :type "Float (single-precision)"))
  (bind _resourcesarray (`self.ResourcesArray`))
  (`KismetSystemLibrary.PrintString` (`KismetStringLibrary.Concat_StrStr` "Health: " (`KismetStringLibrary.Conv_DoubleToString` (`self.Health`)) " \nHunger: " (`KismetStringLibrary.Conv_DoubleToString` (`self.Hunger`)) " \nStamina: " (`KismetStringLibrary.Conv_DoubleToString` (`self.Stamina`)) " \n \nInventory: \n" (`KismetStringLibrary.Conv_IntToString` (`|GetArrayItem` _resourcesarray)) " Wood \n" (`KismetStringLibrary.Conv_IntToString` (`|GetArrayItem` _resourcesarray 1)) " Stone \n" (`KismetStringLibrary.Conv_IntToString` (`|GetArrayItem` _resourcesarray 2)) " Berry")))

(fn `UserConstructionScript`)